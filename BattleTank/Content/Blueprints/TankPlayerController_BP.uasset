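; Player controller Blueprint for a tank that sets up the player's aiming UI.
; On BeginPlay it creates a PlayerUI_BP widget and adds it to the viewport.
; It then passes the widget a small min/max box centered on its crosshair X and Y location variables through SetAimingPosition, placing the aim point on screen.
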(event `self.ReceiveBeginPlay`
  (bind _returnvalue (`|CreateWidget` "/Game/UI/PlayerUI_BP.PlayerUI_BP_C"))
  (`UserWidget.AddToViewport` _returnvalue 0)
  (`/Game/UI/PlayerUI_BP.SetAimingPosition` _returnvalue (- (`self.CrossHairXLocation`) 0.005) (- (`self.CrossHairYLocation`) 0.01) (+ (`self.CrossHairXLocation`) 0.005) (+ (`self.CrossHairYLocation`) 0.01)))

(fn `UserConstructionScript`)